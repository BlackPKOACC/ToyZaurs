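; Roarthur enemy character that roams random reachable points and chases the player once pawn sensing spots them.
; AI Move To drives both states; reaching the player plays an attack animation, then a delayed sphere overlap applies damage, followed by a cooldown.
; Damage lowers health, and a hit taken at zero health plays the death animation and destroys the actor.
; BeginPlay calls the spawner if flagged destroyed; FaceCharacter is never called here.
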(event OnSeePawn(PawnSensing)
  (params (Pawn :type Pawn%20Object%20Reference))
  ;[1 0.04688 0.04688] Chase
  (Variables|Default|SetIs%20Seeing%20Player true)
  (CallFunction|FollowPlayer))

(event Custom|FollowPlayer
  ;[1 0.04688 0.04688] Chase
  (Variables|Default|SetCan%20Attack true)
  (if (Variables|Default|GetIs%20Seeing%20Player)
    (AI|AIMoveTo self "0, 0, 0" (Game|GetPlayerCharacter 0) 1e+01 false
      (:OnSuccess
        (if (Variables|Default|GetCan%20Attack)
          (Variables|Default|SetCan%20Attack false)
          (Components|Animation|PlayAnimation (Variables|Character|GetMesh) "/Game/ToyZaursProject/Characters/Roarthur/Anims/Attack_Roarthur_Anim.Attack_Roarthur_Anim" false)
          (Utilities|FlowControl|Delay 3.29)
          (bind _outactors (Collision|SphereOverlapActors (Transformation|GetWorldLocation (Variables|Default|GetArrow1)) 1e+02 (Variables|Default|GetObject%20Types) 0))
          (Utilities|Array|ForEachLoopwithBreak _outactors :!label _label
            (:LoopBody
              (Game|Damage|ApplyDamage (Game|GetPlayerCharacter 0) (Variables|Default|GetBase%20DMG) 0 0)
              (goto _label Break))
            (:Completed
              (Utilities|FlowControl|Delay 5.0)
              (Variables|Default|SetCan%20Attack true)
              (Components|Animation|SetAnimationMode (Variables|Character|GetMesh) "AnimationBlueprint" true)))))
      (:OnFail
        (CallFunction|Roaming)))))

(event Custom|Roaming
  ;[0.2166 1 0.1624] Roaming
  (AI|AIMoveTo self (.RandomLocation (AI|Navigation|GetRandomReachablePointinRadius (Transformation|GetActorLocation) 1e+04 0 0)) 0 5.0 false
    (:OnSuccess
      (Utilities|FlowControl|Delay (Math|Random|RandomFloatinRange 0.0 0.0))
      (CallFunction|Roaming))))

(event Custom|Face%20Character
  ;[1 0.1822 0.8462] FACE CHARACTER
  (Transformation|SetActorRotation (Math|Rotator|MakeRotator 0.0 0.0 (.yaw (Math|Interpolation|RInterpTo (Transformation|GetActorRotation) (Math|Rotator|FindLookatRotation (Transformation|GetActorLocation) (Transformation|GetActorLocation)) (Utilities|Time|GetWorldDeltaSeconds) 0.0))))
  (Utilities|FlowControl|Delay 0.2)
  (CallFunction|FaceCharacter))

(event EventBeginPlay
  ;[1 0 0.834] Roaming
  (if (Variables|Default|GetIs%20destroyed?)
    (Default|SpawnEnemy (Variables|Default|Getspawner))
    (CallFunction|Roaming)
    (else
      (CallFunction|Roaming))))

(event Game|Damage|EventAnyDamage
  (params (Damage :type Float%20%28single-precision%29) (DamageType :type Damage%20Type%20Object%20Reference) (InstigatedBy :type Controller%20Object%20Reference) (DamageCauser :type Actor%20Object%20Reference))
  ;[0.5 0 1] Health
  (if (> (Variables|Default|GetEnemy%20Health) 0.0)
    (Variables|Default|SetEnemy%20Health (- (Variables|Default|GetEnemy%20Health) Damage))
    (if (<= (Variables|Default|GetEnemy%20Health) 0.0)
      (Variables|Default|SetIs%20destroyed? true)
      (else
        (Variables|Default|SetIs%20destroyed? false)))
    (else
      (Components|Activation|Deactivate (Variables|Character|GetCharacterMovement))
      (Components|Animation|PlayAnimation (Variables|Character|GetMesh) "/Game/ToyZaursProject/Characters/Roarthur/Anims/Death_Roarthur_Anim.Death_Roarthur_Anim" false)
      (Utilities|FlowControl|Delay 2.8)
      (Actor|DestroyActor)
      (Variables|Default|SetDeath true))))

(fn ConstructionScript)