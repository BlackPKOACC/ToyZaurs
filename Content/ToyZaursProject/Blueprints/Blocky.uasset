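; Blocky is a damageable actor that can be destroyed through damage or by an overlap ending.
; Incoming damage reduces BlockyHealth and sets IsDestroyed once health reaches zero or below, but the actor is only removed on the next damage event after that.
; Any end overlap on its Box component destroys it immediately, regardless of health.
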(event OnComponentEndOverlap(Box)
  (params (OverlappedComponent :type Primitive%20Component%20Object%20Reference) (OtherActor :type Actor%20Object%20Reference) (OtherComp :type Primitive%20Component%20Object%20Reference) (OtherBodyIndex :type Integer))
  (Actor|DestroyActor))

(event EventBeginPlay)

(event Collision|EventActorBeginOverlap
  (params (OtherActor :type Actor%20Object%20Reference)))

(event EventTick
  (params (DeltaSeconds :type Float%20%28single-precision%29)))

(event Game|Damage|EventAnyDamage
  (params (Damage :type Float%20%28single-precision%29) (DamageType :type Damage%20Type%20Object%20Reference) (InstigatedBy :type Controller%20Object%20Reference) (DamageCauser :type Actor%20Object%20Reference))
  (if (> (Variables|Default|GetBlocky%20Health) 0.0)
    (Variables|Default|SetBlocky%20Health (- (Variables|Default|GetBlocky%20Health) Damage))
    (if (<= (Variables|Default|GetBlocky%20Health) 0.0)
      (Variables|Default|SetIs%20destroyed? true)
      (else
        (Variables|Default|SetIs%20destroyed? false)))
    (else
      (Actor|DestroyActor))))

(fn ConstructionScript)