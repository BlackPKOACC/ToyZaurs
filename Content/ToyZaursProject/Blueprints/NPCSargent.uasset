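; NPCSargent is an NPC Blueprint that shows dialogue lines one at a time when its Talk event is called.
; Each Talk increments an index into a Dialogue array and writes that line to a WB_DIALOGUE widget, created and added to the viewport if not already valid.
; Past the last line, it removes the widget, clears the reference and resets the index so the conversation can replay.
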(event EventTalk
  (Math|Integer|IncrementInt (Variables|Default|GetTalkindex)
    (:%20%20
      (if (< (Variables|Default|GetTalkindex) (Utilities|Array|Length (Variables|Default|GetDialogue)))
        (Variables|Default|GetUI
          (:then
            _)
          (:else
            (bind _returnvalue (UserInterface|CreateWidget "/Game/ToyZaursProject/BP_IAN/AI/AI_INTERFACE/WB_DIALOGUE.WB_DIALOGUE_C" (Game|GetPlayerController 0)))
            (bind _output_get (Variables|Default|SetUI _returnvalue))
            (UserInterface|Viewport|AddtoViewport _output_get 0)))
        (Rendering|Components|TextRender|SetText (Variables|/Game/ToyZaursProject/BP_IAN/AI/AI_INTERFACE/WB_DIALOGUE.WB_DIALOGUE_C|GetTalkText (Variables|Default|GetUI)) (Utilities|Text|ToText(String) (Utilities|Array|Get(acopy) (Variables|Default|GetDialogue) (Variables|Default|GetTalkindex))))
        (else
          (Widget|RemovefromParent (Variables|Default|GetUI))
          (Variables|Default|SetTalkindex -1)
          (Variables|Default|SetUI 0))))))

(fn ConstructionScript)