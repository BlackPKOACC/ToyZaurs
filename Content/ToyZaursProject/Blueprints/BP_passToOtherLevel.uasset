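; BP_passToOtherLevel is a level exit trigger that sends Trixie to the Roarthur level once all items are collected.
; Its Collectitem event increments the collected count and, at the maximum, reaches a DoOnce with nothing after it.
; When Trixie overlaps the Box, it opens RoarthurLevel by object reference only if the count exactly equals the maximum.
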(event OnComponentBeginOverlap(Box)
  (params (OverlappedComponent :type Primitive%20Component%20Object%20Reference) (OtherActor :type Actor%20Object%20Reference) (OtherComp :type Primitive%20Component%20Object%20Reference) (OtherBodyIndex :type Integer) (bFromSweep :type Boolean) (SweepResult :type Hit%20Result%20Structure%20%28by%20ref%29))
  (Utilities|Casting|CastToTrixie OtherActor)
  (if true
    (if (== (Variables|Default|GetCurrentItemsCollected) (Variables|Default|GetMaxItemsCollected))
      (Game|OpenLevel(byObjectReference) "/Game/ToyZaursProject/Levels/RoarthurLevel.RoarthurLevel"))))

(event Custom|Collect%20item
  (Math|Integer|IncrementInt (Variables|Default|GetCurrentItemsCollected)
    (:%20%20
      (if (>= (Variables|Default|GetCurrentItemsCollected) (Variables|Default|GetMaxItemsCollected))
        (Utilities|FlowControl|DoOnce false)))))

(fn ConstructionScript)