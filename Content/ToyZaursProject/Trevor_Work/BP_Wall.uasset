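; BP_Wall is a wall actor that raises and lowers its static mesh in response to a BP_Button.
; On BeginPlay it finds a single BP_Button via GetActorOfClass and binds its open and close events.
; Open and Close use eased MoveComponentTo to shift the mesh 500 units up or down, feeding an offset world location in as the relative target.
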(event Custom|Open
  (bind _staticmesh (Variables|Default|GetStaticMesh))
  (Components|MoveComponentTo _staticmesh (+ (Transformation|GetWorldLocation _staticmesh) "0.000000,0.000000,500.000000") "0, 0, 0" true true 0.2 false))

(event Custom|Close
  (bind _staticmesh (Variables|Default|GetStaticMesh))
  (Components|MoveComponentTo _staticmesh (+ (Transformation|GetWorldLocation _staticmesh) "0.000000,0.000000,-500.000000") "0, 0, 0" true true 0.2 false))

(event EventBeginPlay
  (bind _returnvalue (Actor|GetActorOfClass "/Game/ToyZaursProject/Trevor_Work/BP_Button.BP_Button_C"))
  (bind _output_get (Variables|Default|SetButton _returnvalue))
  (EventDispatchers|BindEventtoOpen _output_get (delegate Custom|Open))
  (EventDispatchers|BindEventtoClose _output_get (delegate Custom|Close)))

(fn ConstructionScript)